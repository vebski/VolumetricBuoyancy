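; Helper functions for point-based buoyancy, floating physics objects on the waves of an ocean manager.
; EvalWaveHeightAtPoint moves a local point to world space, samples wave height, and returns submersion state, depth and a cubed, clamped force factor based on point thickness.
; ProcessWaveHeightAtPoint uses that factor to apply upward displacement force when submerged or downward gravity-like force otherwise, at that point on the component, with always-on debug arrows and spheres.
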(fn EvalWaveHeightatPoint
  (params (PointLocation :type Vector) (ActorTransform :type Transform) (OceanManager :type Ocean%20Manager%20Object%20Reference) (PointThickness :type Float%20%28single-precision%29) (Time :type Float%20%28single-precision%29))
  (bind _returnvalue (Math|Transform|TransformLocation ActorTransform PointLocation))
  (bind _z (Math|Vector|BreakVector _returnvalue))
  (bind _returnvalue_2 (Class|OceanManager|GetWaveHeight OceanManager _returnvalue Time))
  (return (> (- (.Z (Math|Vector|BreakVector _returnvalue_2)) _z) 0.0) (Math|Float|Absolute(Float) (Math|Float|Clamp(Float) (Math|Float|Power (/ (- (.Z (Math|Vector|BreakVector _returnvalue_2)) _z) PointThickness) 3.0) -1.0)) (- (.Z (Math|Vector|BreakVector _returnvalue_2)) _z) (Math|Vector|MakeVector (.X (Math|Vector|BreakVector (+ _returnvalue _returnvalue_2))) (.Y (Math|Vector|BreakVector (+ _returnvalue _returnvalue_2))) _z) (.Z (Math|Vector|BreakVector _returnvalue_2))))

(fn ProcessWaveHeightatPoint
  (params (PointLocation :type Vector) (PrimitiveComponent :type Primitive%20Component%20Object%20Reference) (OceanManager :type Ocean%20Manager%20Object%20Reference) (ActorTransform :type Transform) (MassOfPoint :type Float%20%28single-precision%29) (PointThickness :type Float%20%28single-precision%29) (DisplacementRatio :type Float%20%28single-precision%29) (Time :type Float%20%28single-precision%29))
  (bind _returnvalue (Class|KismetSystemLibrary|MakeLiteralBool true))
  (bind _returnvalue_2 (Math|Transform|TransformLocation ActorTransform PointLocation))
  (bind (_isunder _amount) (CallFunction|EvalWaveHeightatPoint PointLocation ActorTransform OceanManager PointThickness Time))
  (if _isunder
    (Class|PrimitiveComponent|AddForceatLocation PrimitiveComponent (* (* (Math|Vector|MakeVector 0.0 0.0 (* DisplacementRatio 9.8e+02)) MassOfPoint) _amount) _returnvalue_2 "None")
    (if _returnvalue
      ;[1 1 1] Draw Debug Helpers
      (Rendering|Debug|DrawDebugArrow 0 _returnvalue_2 (+ _returnvalue_2 "0, 0,25.000000") 15.0 "(R=1.000000,G=0.887112,B=0.000000,A=1.000000)" 0.0)
      (Rendering|Debug|DrawDebugSphere 0 _returnvalue_2 1e+01 12 "(R=1.000000,G=0.000000,B=0.017573,A=1.000000)" :!label _label))
    (else
      (Class|PrimitiveComponent|AddForceatLocation PrimitiveComponent (* (* (Math|Vector|MakeVector 0.0 0.0 -9.8e+02) MassOfPoint) _amount) _returnvalue_2 "None")
      (if _returnvalue
        (Rendering|Debug|DrawDebugArrow 0 _returnvalue_2 (+ _returnvalue_2 "0, 0,-25.000000") 15.0 "(R=1.000000,G=0.864500,B=0.000000,A=1.000000)" 0.0)
        (goto _label)
        (else
          _))))
  (return _isunder))